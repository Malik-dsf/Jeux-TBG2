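; BP_IAClassique is a basic AI pawn that chases the player and can be killed.
; When PawnSensing sees a ThirdPersonCharacter, AIMoveTo sends the pawn toward it.
; DamageIA subtracts point damage from VieIA and calls MortIA once health is no longer above zero.
; MortIA only plays a 2D explosion sound, without destroying or disabling the pawn.
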(event OnSeePawn(PawnSensing)
  (params (Pawn :type Pawn%20Object%20Reference))
  (bind _asthird_person_character (Utilities|Casting|CastToThirdPersonCharacter Pawn))
  (AI|AIMoveTo self "0, 0, 0" _asthird_person_character 5.0 false))

(event EventBeginPlay)

(event Collision|EventActorBeginOverlap
  (params (OtherActor :type Actor%20Object%20Reference)))

(event EventTick
  (params (DeltaSeconds :type Float%20%28single-precision%29)))

(fn ConstructionScript)

(fn DamageIA
  (params (PointDamage :type Float%20%28single-precision%29))
  (Variables|Default|SetvieIA (- (Variables|Default|GetvieIA) PointDamage))
  (if (not (> (Variables|Default|GetvieIA) 0.0))
    (CallFunction|MortIA)))

(fn MortIA
  (Audio|PlaySound2D "/Game/StarterContent/Audio/Explosion01.Explosion01" 1.0 1.0 0.0 0 0))