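; BP_Fumertue is an item that deals damage over time to a ThirdPersonCharacter that enters its Box.
; The overlap stores the character and starts a looping one-second timer.
; Each tick subtracts Pointdamages from Health, clamped between zero and HeathMax, and increments Compteur until it reaches Duree, when the timer is cleared.
; Compteur is never reset here, so the tick budget is shared across all overlaps.
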(event OnComponentBeginOverlap(Box)
  (params (OverlappedComponent :type Primitive%20Component%20Object%20Reference) (OtherActor :type Actor%20Object%20Reference) (OtherComp :type Primitive%20Component%20Object%20Reference) (OtherBodyIndex :type Integer) (bFromSweep :type Boolean) (SweepResult :type Hit%20Result%20Structure%20%28by%20ref%29))
  (bind _asthird_person_character (Utilities|Casting|CastToThirdPersonCharacter OtherActor))
  (CallFunction|Damage))

(event Custom|damage
  (bind _returnvalue (Utilities|Time|SetTimerbyEvent (delegate Custom|infligerdamage) 1.0 true)))

(event Custom|infligerdamage
  (if (< (Variables|Default|Getcompteur) (Variables|Default|Getduree))
    (Variables|/Game/ThirdPersonBP/Blueprints/ThirdPersonCharacter.ThirdPersonCharacter_C|SetHealth (stale OnComponentBeginOverlap(Box) _asthird_person_character) (Math|Float|Clamp(Float) (- (Variables|/Game/ThirdPersonBP/Blueprints/ThirdPersonCharacter.ThirdPersonCharacter_C|GetHealth (stale OnComponentBeginOverlap(Box) _asthird_person_character)) (Variables|Default|Getpointdamages)) 0.0 (Variables|/Game/ThirdPersonBP/Blueprints/ThirdPersonCharacter.ThirdPersonCharacter_C|GetHeathMax (stale OnComponentBeginOverlap(Box) _asthird_person_character))))
    (Math|Integer|IncrementInt (Variables|Default|Getcompteur))
    (else
      (Utilities|Time|ClearandInvalidateTimerbyHandle (stale Custom|damage _returnvalue)))))

(event EventBeginPlay)

(event Collision|EventActorBeginOverlap
  (params (OtherActor :type Actor%20Object%20Reference)))

(event EventTick
  (params (DeltaSeconds :type Float%20%28single-precision%29)))

(fn ConstructionScript)